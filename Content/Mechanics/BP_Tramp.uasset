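; BP_Tramp is a trampoline-style trigger that launches the ball and awards points on contact.
; When a BP_Ball overlaps its Box, it applies an impulse to the ball's Sphere along the Box's forward vector, scaled by ImpulseForce.
; It then adds ScoreValue to CurrentScore in the VariableStorage game instance.
; The impulse is not a velocity change, so the ball's mass affects the launch speed.
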(event OnComponentBeginOverlap(Box)
  (params (OverlappedComponent :type Primitive%20Component%20Object%20Reference) (OtherActor :type Actor%20Object%20Reference) (OtherComp :type Primitive%20Component%20Object%20Reference) (OtherBodyIndex :type Integer) (bFromSweep :type Boolean) (SweepResult :type Hit%20Result%20Structure%20%28by%20ref%29))
  (bind _asbp_ball (Utilities|Casting|CastToBP_Ball OtherActor))
  (Physics|AddImpulse (Variables|/Game/Mechanics/BP_Ball.BP_Ball_C|GetSphere _asbp_ball) (* (Math|Vector|GetForwardVector (Variables|Default|GetBox)) (Variables|Default|GetImpulseForce)) "None" false)
  (bind _asvariable_storage (Utilities|Casting|CastToVariableStorage (Game|GetGameInstance)))
  (Variables|/Game/Logic/VariableStorage.VariableStorage_C|SetCurrentScore _asvariable_storage (+ (Variables|/Game/Logic/VariableStorage.VariableStorage_C|GetCurrentScore _asvariable_storage) (Variables|Default|GetScoreValue))))

(fn ConstructionScript)